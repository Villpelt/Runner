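; Vuorovaikutus (Finnish for "interaction") is an actor for a moving collectible, shifted each Tick by Nopeus scaled by global time dilation, not delta time.
; Helper functions reset its position at a random height and randomize its scale, deriving the value Arvo from that scale.
; Name comparisons detect hits on the player character or respawn trigger.
; Overlap and Efekti are empty, and nothing here calls the helpers.
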(event EventBeginPlay)

(event Collision|EventActorBeginOverlap
  (params (OtherActor :type Actor%20Object%20Reference)))

(event EventTick
  (params (DeltaSeconds :type Float%20%28single-precision%29))
  ;[1 1 1] Liikuttaa kerättävää
  (Transformation|AddActorWorldOffset (* (Variables|Default|GetNopeus) (Class|GameplayStatics|GetGlobalTimeDilation))))

(fn ConstructionScript)

(fn ResetPositio
  (bind _alkupositio (Variables|Default|GetAlkuPositio))
  (bind (_x _y) (Math|Vector|BreakVector _alkupositio))
  (Transformation|SetActorLocation (Math|Vector|MakeVector _x _y (Math|Random|RandomFloatinRange 4e+02 7.5e+02)) false false))

(fn ResetSkaalaJaArvo
  (bind _output_get (Variables|Default|SetSkaala (Math|Random|RandomFloatinRange 1.0 4.0)))
  (Transformation|SetActorScale3D (Math|Vector|MakeVector (/ _output_get 2.0) (/ _output_get 2.0) (/ _output_get 2.0)))
  (Variables|Default|SetArvo (Math|Float|Round (Variables|Default|GetSkaala))))

(fn HugoOsuma
  (params (ToinenEsine :type String))
  (return (Utilities|Enum|Equal(Enum) ToinenEsine (Utilities|GetObjectName (Game|GetPlayerCharacter 0)))))

(fn RespawnOsuma
  (params (ToinenEsine :type String))
  (return (Utilities|Enum|Equal(Enum) ToinenEsine (Variables|Default|GetRespawnTriggerNimi))))

(fn Efekti)