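; Hugo is a Paper2D player character blueprint with a jump input and a flipbook sprite.
; BeginPlay sets game-only input, and the Hyppy action makes player character 0 jump.
; Capsule hits on actors tagged "Pinta" (surface) switch the sprite to the Kävely (walk) flipbook.
; The left and right axis events are empty, with their AddMovementInput nodes left unconnected, so they move nothing.
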(event OnComponentHit(CapsuleComponent)
  (params (HitComponent :type Primitive%20Component%20Object%20Reference) (OtherActor :type Actor%20Object%20Reference) (OtherComp :type Primitive%20Component%20Object%20Reference) (NormalImpulse :type Vector :default "0, 0, 0") (Hit :type Hit%20Result%20Structure%20%28by%20ref%29))
  (if (Actor|ActorHasTag OtherActor "Pinta")
    (Sprite|SetFlipbook (Variables|Default|GetSprite) "/Game/Flipbooks/Kävely.Kävely")))

(event EventBeginPlay
  (Input|SetInputModeGameOnly (Game|GetPlayerController 0)))

(event Collision|EventActorBeginOverlap
  (params (OtherActor :type Actor%20Object%20Reference)))

(event EventTick
  (params (DeltaSeconds :type Float%20%28single-precision%29)))

(event Input|ActionEvents|InputActionHyppy
  (params (Key :type Key%20Structure :default "None"))
  (:Pressed
    (Character|Jump (Game|GetPlayerCharacter 0))))

(event Input|AxisEvents|InputAxisLiiku_oikealle
  (params (AxisValue :type Float%20%28single-precision%29))
  ;[1 1 1] Toteuttaa liikkumisen oikealle ja vasemmalle
)

(event Input|AxisEvents|InputAxisLiiku_vasemmalle
  (params (AxisValue :type Float%20%28single-precision%29))
  ;[1 1 1] Toteuttaa liikkumisen oikealle ja vasemmalle
)

(fn ConstructionScript)